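; Camera actor that acts as the player in an on-rails shooter, riding a track while the player clicks to shoot.
; When active, a timeline moves it along the referenced track's spline over a set duration, then shows a results widget with a sound.
; Clicks trace under the cursor, spawn an explosion and damage any BasicEnemy hit.
; TakeHit drains player health and returns to the Title level at zero, as does Escape.
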(event `self.ReceiveBeginPlay`
  (if (`self.ActiveCart`)
    (`self.MoveCart`)
    (`self.EnableInput` (`GameplayStatics.GetPlayerController` 0))))

(event `Key|Escape`
  (params (Key :type "Key Structure"))
  (:`Pressed`
    (`GameplayStatics.OpenLevel` "Title")))

(event `MoveCart`
  (bind _returnvalue (`KismetMathLibrary.Lerp` 0.0 (`SplineComponent.GetSplineLength` (`/Game/Blueprints/Track_Blueprint.UsefulSpline` (`self.TrackReference`))) (`self.Alpha`)))
  (`TimelineComponent.SetPlayRate` (`self.CameraMover`) (/ 1.0 (`self.Duration`)))
  (`TimelineComponent.SetNewTime` (`self.CameraMover`) (`self.CartStartOffset`))
  (bind (_direction _newtrack_0) (`Timeline|CameraMover`)
    (:`Update`
      (set `self.Alpha` _newtrack_0)
      (`self.K2_SetActorLocationAndRotation` (`SplineComponent.GetLocationAtDistanceAlongSpline` (`/Game/Blueprints/Track_Blueprint.UsefulSpline` (`self.TrackReference`)) _returnvalue "World") (`SplineComponent.GetRotationAtDistanceAlongSpline` (`/Game/Blueprints/Track_Blueprint.UsefulSpline` (`self.TrackReference`)) _returnvalue "World")))
    (:`Finished`
      (bind _returnvalue_2 (`|CreateWidget` "/Game/UserAssets/UI/Results.Results_C"))
      (`UserWidget.AddToViewport` _returnvalue_2 0)
      (`GameplayStatics.PlaySound2D` "/Game/UserAssets/Audio/BMAD_results.BMAD_results" 1.0 1.0 0.0 null null))))

(event `Key|LeftMouseButton`
  (params (Key :type "Key Structure"))
  (:`Pressed`
    (`self.LineTrace`)))

(event `LineTrace`
  (bind (_bblockinghit _binitialoverlap _time _distance _location _impactpoint _normal _impactnormal _physmat _hitactor) (`GameplayStatics.BreakHitResult` (`PlayerController.GetHitResultUnderCursorByChannel` (`GameplayStatics.GetPlayerController` 0) "TraceTypeQuery1" true)))
  (`GameplayStatics.SpawnEmitterAtLocation` "/Game/StarterContent/Particles/P_Explosion.P_Explosion" _location)
  (`GameplayStatics.PlaySound2D` "/Game/StarterContent/Audio/Explosion_Cue.Explosion_Cue" 1.0 1.0 0.0 null null)
  (bind _output_get (set `self.Hit Actor` _hitactor))
  (bind _asbasic_enemy (cast `/Game/Blueprints/BasicEnemy` _output_get))
  (set `/Game/Blueprints/BasicEnemy.Health` (- (`/Game/Blueprints/BasicEnemy.Health` _asbasic_enemy) 1) _asbasic_enemy)
  (`/Game/Blueprints/BasicEnemy.Death Check` _asbasic_enemy))

(event `TakeHit`
  (bind _output_get (set `self.PlayerHealth` (- (`self.PlayerHealth`) 1)))
  (if (<= _output_get 0)
    (`GameplayStatics.OpenLevel` "Title")))

(fn `UserConstructionScript`)
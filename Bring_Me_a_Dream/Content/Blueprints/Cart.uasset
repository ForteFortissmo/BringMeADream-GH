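; Cart actor that rides along the spline of a referenced track actor.
; On BeginPlay, if the cart is active, it starts a timeline with play rate set from Duration and start time set from an offset.
; Each timeline update maps Alpha to a distance along the spline and sets the cart's world location and rotation to match that point.
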(event `self.ReceiveBeginPlay`
  (if (`self.ActiveCart`)
    (`self.MoveCart`)))

(event `MoveCart`
  (bind _returnvalue (`KismetMathLibrary.Lerp` 0.0 (`SplineComponent.GetSplineLength` (`/Game/Blueprints/Track_Blueprint.UsefulSpline` (`self.TrackReference`))) (`self.Alpha`)))
  (`TimelineComponent.SetPlayRate` (`self.CartMover`) (/ 1.0 (`self.Duration`)))
  (`TimelineComponent.SetNewTime` (`self.CartMover`) (`self.CartStartOffset`))
  (bind (_direction _alpha) (`Timeline|CartMover`)
    (:`Update`
      (set `self.Alpha` _alpha)
      (`self.K2_SetActorLocationAndRotation` (`SplineComponent.GetLocationAtDistanceAlongSpline` (`/Game/Blueprints/Track_Blueprint.UsefulSpline` (`self.TrackReference`)) _returnvalue "World") (`SplineComponent.GetRotationAtDistanceAlongSpline` (`/Game/Blueprints/Track_Blueprint.UsefulSpline` (`self.TrackReference`)) _returnvalue "World")))))

(fn `UserConstructionScript`)